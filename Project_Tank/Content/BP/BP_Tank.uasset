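; BP_Tank is a player-controlled tank Blueprint with a turret, cannon, two independently driven tracks and an orbiting camera rig.
; On BeginPlay it passes the barrel and turret to the Aiming component and the barrel to itself.
; Azimuth and altitude axes yaw the Scene component and pitch the SpringArm.
; Separate left and right axes send movement requests to their tracks, and the Fire action calls Spara to shoot.
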(event `self.ReceiveBeginPlay`
  (bind _aiming (`self.Aiming`))
  (bind _barrell (`self.Barrell`))
  (`Aiming_C.SetCannone` _aiming _barrell)
  (`Aiming_C.SetTorretta` _aiming (`self.Torretta`))
  (`self.SetCannone` _barrell))

(event `InputAction|Fire`
  (params (Key :type "Key Structure"))
  (:`Pressed`
    (`self.Spara`)))

(event `InputAxis|MoveAltitude`
  (params (AxisValue :type "Float (single-precision)"))
  (`SceneComponent.K2_AddLocalRotation` (`self.SpringArm`) (`KismetMathLibrary.MakeRotator` 0.0 AxisValue) false false))

(event `InputAxis|MoveAzimut`
  (params (AxisValue :type "Float (single-precision)"))
  (`SceneComponent.K2_AddLocalRotation` (`self.Scene`) (`KismetMathLibrary.MakeRotator` 0.0 0.0 AxisValue) false false))

(event `InputAxis|MoveForwardTrack_SX`
  (params (AxisValue :type "Float (single-precision)"))
  (`Mesh_Cingolo.RichiestaMovimento` (`self.Cingolo_SX`) AxisValue))

(event `InputAxis|MoveForwardTrack_DX`
  (params (AxisValue :type "Float (single-precision)"))
  (`Mesh_Cingolo.RichiestaMovimento` (`self.Cingolo_DX`) AxisValue))

(fn `UserConstructionScript`)